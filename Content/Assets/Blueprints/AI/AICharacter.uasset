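; AI character that reacts to the player and picks up a dummy object through its TouchBox overlap.
; Player overlap disables the player's movement until overlap ends, with debug prints.
; If the first BP_Dummy overlaps while the game mode's dummy state is set, GrabObject attaches a runtime-created physics handle, ignores Pawn collision and clears that state.
; Tick then moves the handle to LocalSocket; GiveObject is an empty stub.
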(event OnComponentEndOverlap(TouchBox)
  (params (OverlappedComponent :type Primitive%20Component%20Object%20Reference) (OtherActor :type Actor%20Object%20Reference) (OtherComp :type Primitive%20Component%20Object%20Reference) (OtherBodyIndex :type Integer))
  (if (== OtherActor (Game|GetPlayerCharacter 0))
    (bind _asplayer_character (Utilities|Casting|CastToPlayerCharacter OtherActor))
    (Development|PrintString "Buy")
    (Class|PlayerCharacter|SetCanMove _asplayer_character true)))

(event OnComponentBeginOverlap(TouchBox)
  (params (OverlappedComponent :type Primitive%20Component%20Object%20Reference) (OtherActor :type Actor%20Object%20Reference) (OtherComp :type Primitive%20Component%20Object%20Reference) (OtherBodyIndex :type Integer) (bFromSweep :type Boolean) (SweepResult :type Hit%20Result%20Structure%20%28by%20ref%29))
  (if (== OtherActor (Game|GetPlayerCharacter 0))
    (bind _asplayer_character (Utilities|Casting|CastToPlayerCharacter OtherActor))
    (Development|PrintString "Hello")
    (Class|PlayerCharacter|SetCanMove _asplayer_character false)
    (else
      (bind _outactors (Actor|GetAllActorsOfClass "/Game/Assets/Blueprints/BP_Dummy.BP_Dummy_C"))
      (if (== OtherActor (Utilities|Array|Get(acopy) _outactors))
        (bind _asbp_aiproject_game_mode_base (Utilities|Casting|CastToBP_AIProjectGameModeBase (Game|GetGameMode)))
        (bind _dummystate (Default|GetDummyState _asbp_aiproject_game_mode_base))
        (if _dummystate
          (CallFunction|GrabObject OtherComp))))))

(event EventBeginPlay)

(event Collision|EventActorBeginOverlap
  (params (OtherActor :type Actor%20Object%20Reference)))

(event EventTick
  (params (DeltaSeconds :type Float%20%28single-precision%29))
  (if (Variables|Default|GetisHandled)
    (CallFunction|UpdatePhysics)))

(fn ConstructionScript)

(fn GrabObject
  (params (NewParam :type Primitive%20Component%20Object%20Reference))
  (bind _returnvalue (AddComponent|AddPhysicsHandleComponent (Transformation|GetActorTransform)))
  (Variables|Default|SetPhysicsHandle _returnvalue)
  (Variables|Default|SetPhysicsObject NewParam)
  (Class|PhysicsHandleComponent|GrabComponentatLocation (Variables|Default|GetPhysicsHandle) NewParam "None" (Transformation|GetWorldLocation NewParam))
  (Collision|SetCollisionResponsetoChannel NewParam "ECC_Pawn" "ECR_Ignore")
  (bind _asbp_aiproject_game_mode_base (Utilities|Casting|CastToBP_AIProjectGameModeBase (Game|GetGameMode)))
  (Default|SetDummyState _asbp_aiproject_game_mode_base false)
  (Variables|Default|SetisHandled true))

(fn UpdatePhysics
  (Physics|Components|PhysicsHandle|SetTargetLocation (Variables|Default|GetPhysicsHandle) (Transformation|GetWorldLocation (Variables|Default|GetLocalSocket))))

(fn GiveObject)